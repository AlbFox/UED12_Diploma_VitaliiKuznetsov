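; Base weapon Blueprint that handles automatic firing of BP_BaseBullet projectiles from its muzzle component.
; MakeShot fires at once and starts a looping timer at the AttacksPerSecond interval, which StopShooting clears.
; SpawnShot checks and spends ammo through the assigned weapon component, then spawns BulletsPerShot bullets configured from AttackParameters.
; IsReloading acts as a between-shot cooldown that blocks new MakeShot calls, rather than a magazine refill.
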(event `MakeShot`
  (if (not (`self.IsReloading`))
    (`self.SpawnShot`)
    (bind _returnvalue (`KismetSystemLibrary.K2_SetTimerDelegate` (`|CreateDelegate` :!event `SpawnShot`) (`self.CalculateFireRate` (`.AttacksPerSecond_2_DB57C88D4ED29087BF49F99CDCB5527A` (break `/Game/Blueprints/Components/Weapon/Str_AttackParameters` (`self.AttackParameters`)))) true))
    (set `self.SpawnShotHandle` _returnvalue)))

(event `StopShooting`
  (`KismetSystemLibrary.K2_ClearAndInvalidateTimerHandle` (`self.SpawnShotHandle`)))

(fn `CalculateFireRate`
  (params (AttacksPerSecond :type "Float (double-precision)"))
  (returns (ReturnValue :type "Float (double-precision)"))
  (if (!= AttacksPerSecond 0.0)
    (return (/ 1.0 AttacksPerSecond))))

(fn `Reloading`
  (set `self.IsReloading` false))

(fn `SetComponentWeapon`
  (params (ComponentWeapon :type "/Game/Blueprints/Components/Weapon/Comp_Weapon Object Reference"))
  (set `self.ComponentWeapon` ComponentWeapon))

(fn `SpawnBullet`
  (params (AttackParameters :type "/Game/Blueprints/Components/Weapon/Str_AttackParameters Structure"))
  (locals (L_AttackParameters :type "/Game/Blueprints/Components/Weapon/Str_AttackParameters Structure"))
  (bind (_l_attackparameters_attackspersecond _l_attackparameters_zspread _l_attackparameters_bulletspershot _l_attackparameters_damage _l_attackparameters_bulletspeed _l_attackparameters_bulletlifetime) (break `/Game/Blueprints/Components/Weapon/Str_AttackParameters` (`local.L_AttackParameters`)))
  (set `local.L_AttackParameters` AttackParameters)
  (for _ (range 1 (+ _l_attackparameters_bulletspershot 1))
    (`|SpawnActorFromClass` "/Game/Blueprints/Components/Weapon/BP_BaseBullet.BP_BaseBullet_C" (`KismetMathLibrary.MakeTransform` (`SceneComponent.K2_GetComponentLocation` (`self.SComp_Muzzle`))) "Undefined" "OverrideRootScale" null _l_attackparameters_damage _l_attackparameters_bulletspeed _l_attackparameters_bulletlifetime null)))

(fn `SpawnShot`
  (bind _attackparameters (`self.AttackParameters`))
  (if (`/Game/Blueprints/Components/Weapon/Comp_Weapon.CheckWeaponCurrentAmmo` (`self.ComponentWeapon`) (`self.WeaponName`))
    (`/Game/Blueprints/Components/Weapon/Comp_Weapon.DecreaseWeaponCurrentAmmo` (`self.ComponentWeapon`) (`self.WeaponName`))
    (`self.SpawnBullet` _attackparameters)
    (set `self.IsReloading` true)
    (`KismetSystemLibrary.K2_SetTimerDelegate` (`|CreateDelegate` :!event `Reloading`) (`self.CalculateFireRate` (`.AttacksPerSecond_2_DB57C88D4ED29087BF49F99CDCB5527A` (break `/Game/Blueprints/Components/Weapon/Str_AttackParameters` _attackparameters))))))

(fn `UserConstructionScript`)