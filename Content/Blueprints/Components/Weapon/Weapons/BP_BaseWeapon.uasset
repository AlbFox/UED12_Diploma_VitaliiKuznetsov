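; Base weapon that fires projectile bullets for the player, either single or multiple per shot.
; MakeShot fires immediately and starts a looping fire-rate timer until StopShooting, with IsReloading acting as a between-shot cooldown.
; SpawnShot checks and decrements ammo through the weapon component, then spawns BP_BaseBullet actors from the muzzle.
; Bullets aim at a camera trace hit point, randomly offset by weapon spread, which widens when not aiming.
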(event `self.ReceiveBeginPlay`
  (bind _asbp_player_character (cast `/Game/Player/Blueprints/BP_PlayerCharacter` (`GameplayStatics.GetPlayerCharacter` 0)))
  (set `self.PlayerCharacter` _asbp_player_character))

(event `StopShooting`
  (`KismetSystemLibrary.K2_ClearAndInvalidateTimerHandle` (`self.SpawnShotHandle`)))

(event `MakeShot`
  (if (not (`self.IsReloading`))
    (`self.SpawnShot`)
    (bind _returnvalue (`KismetSystemLibrary.K2_SetTimerDelegate` (`|CreateDelegate` :!event `SpawnShot`) (`self.CalculateFireRate` (`.AttacksPerSecond_2_DB57C88D4ED29087BF49F99CDCB5527A` (break `/Game/Blueprints/Components/Weapon/ComponentWeapons/Str_AttackParameters` (`self.AttackParameters`)))) true))
    (set `self.SpawnShotHandle` _returnvalue)))

(fn `CalculateFireRate`
  (params (AttacksPerSecond :type "Float (double-precision)"))
  (returns (ReturnValue :type "Float (double-precision)"))
  (if (!= AttacksPerSecond 0.0)
    (return (/ 1.0 AttacksPerSecond))))

(fn `CalculateProjectileRotAndLoc`
  (returns (SpreadLocation :type "Vector Structure") (SpreadRotation :type "Rotator Structure"))
  (bind _returnvalue (`SceneComponent.K2_GetComponentLocation` (`self.SComp_Muzzle`)))
  (bind _camera (`/Game/Player/Blueprints/BP_PlayerCharacter.Camera` (`self.PlayerCharacter`)))
  (bind _returnvalue_2 (`SceneComponent.K2_GetComponentLocation` _camera))
  (bind _outhit (`KismetSystemLibrary.LineTraceSingle` :`Start` _returnvalue_2 :`End` (+ (* (`SceneComponent.GetForwardVector` _camera) 10000.0) _returnvalue_2) :`TraceChannel` "TraceTypeQuery1" :`DrawDebugType` "ForOneFrame"))
  (return _returnvalue (`KismetMathLibrary.FindLookAtRotation` _returnvalue (`self.CalculateSpread` (`.Location` (`GameplayStatics.BreakHitResult` _outhit))))))

(fn `CalculateSpread`
  (params (VectorToModify :type "Vector Structure"))
  (returns (ModifiedVector :type "Vector Structure"))
  (return (`KismetMathLibrary.MakeVector` (+ (.x VectorToModify) (`self.GetSpread`)) (+ (.y VectorToModify) (`self.GetSpread`)) (+ (.z VectorToModify) (`self.GetSpread`)))))

(fn `GetSpread`
  (returns (RandomSpread :type "Float (double-precision)"))
  (bind _returnvalue (* (+ (`.ZSpread_4_6097731E47F24CAFE8117EBA5E8CA805` (break `/Game/Blueprints/Components/Weapon/ComponentWeapons/Str_AttackParameters` (`self.AttackParameters`))) (`KismetMathLibrary.SelectFloat` 0.0 90.0 (`/Game/Player/Blueprints/BP_PlayerCharacter.IsAiming` (`self.PlayerCharacter`)))) 0.5))
  (return (`KismetMathLibrary.RandomFloatInRange` (* _returnvalue -1.0) _returnvalue)))

(fn `Reloading`
  (set `self.IsReloading` false))

(fn `SetComponentWeapon`
  (params (ComponentWeapon :type "/Game/Blueprints/Components/Weapon/ComponentWeapons/Comp_Weapon Object Reference"))
  (set `self.ComponentWeapon` ComponentWeapon))

(fn `SpawnBullet`
  (params (AttackParameters :type "/Game/Blueprints/Components/Weapon/ComponentWeapons/Str_AttackParameters Structure"))
  (locals (L_AttackParameters :type "/Game/Blueprints/Components/Weapon/ComponentWeapons/Str_AttackParameters Structure"))
  (bind (_spreadlocation _spreadrotation) (`self.CalculateProjectileRotAndLoc`))
  (bind (_l_attackparameters_attackspersecond _l_attackparameters_zspread _l_attackparameters_bulletspershot _l_attackparameters_damage _l_attackparameters_bulletspeed _l_attackparameters_bulletlifetime) (break `/Game/Blueprints/Components/Weapon/ComponentWeapons/Str_AttackParameters` (`local.L_AttackParameters`)))
  (set `local.L_AttackParameters` AttackParameters)
  (for _ (range 1 (+ _l_attackparameters_bulletspershot 1))
    (`|SpawnActorFromClass` "/Game/Blueprints/Components/Weapon/Weapons/BP_BaseBullet.BP_BaseBullet_C" (`KismetMathLibrary.MakeTransform` _spreadlocation _spreadrotation (0.4 0.4 0.4)) "Undefined" "OverrideRootScale" null _l_attackparameters_damage _l_attackparameters_bulletspeed _l_attackparameters_bulletlifetime null)))

(fn `SpawnShot`
  (bind _attackparameters (`self.AttackParameters`))
  (if (`/Game/Blueprints/Components/Weapon/ComponentWeapons/Comp_Weapon.CheckWeaponCurrentAmmo` (`self.ComponentWeapon`) (`self.WeaponName`))
    (`/Game/Blueprints/Components/Weapon/ComponentWeapons/Comp_Weapon.DecreaseWeaponCurrentAmmo` (`self.ComponentWeapon`) (`self.WeaponName`))
    (`self.SpawnBullet` _attackparameters)
    (set `self.IsReloading` true)
    (`KismetSystemLibrary.K2_SetTimerDelegate` (`|CreateDelegate` :!event `Reloading`) (`self.CalculateFireRate` (`.AttacksPerSecond_2_DB57C88D4ED29087BF49F99CDCB5527A` (break `/Game/Blueprints/Components/Weapon/ComponentWeapons/Str_AttackParameters` _attackparameters))))))

(fn `UserConstructionScript`)