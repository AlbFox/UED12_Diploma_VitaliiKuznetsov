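; BP_RocketExplosion is a short-lived damage volume that deals area damage for a rocket explosion.
; Its Sphere collects overlapping actors into a unique list, and both BeginPlay and each overlap schedule DealDamageInArea after a short delay.
; DealDamageInArea sends DealDamageMessage with a fixed amount to every collected actor, then destroys the volume.
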(event `self.ReceiveBeginPlay`
  (`KismetSystemLibrary.Delay` 0.2)
  (`self.DealDamageInArea`))

(event `self.Sphere.OnComponentBeginOverlap`
  (params (OverlappedComponent :type "PrimitiveComponent Object Reference") (OtherActor :type "Actor Object Reference") (OtherComp :type "PrimitiveComponent Object Reference") (OtherBodyIndex :type Integer) (bFromSweep :type Boolean) (SweepResult :type "HitResult Structure (by ref)"))
  (`KismetArrayLibrary.Array_AddUnique` (`self.ActorsToDamage`) OtherActor)
  (`KismetSystemLibrary.Delay` 0.2)
  (`self.DealDamageInArea`))

(fn `DealDamageInArea`
  (for _array_element (`self.ActorsToDamage`)
    (message `/Game/Blueprints/Components/Parameters/BPI_Damage.DealDamage` _array_element 100))
  (`self.K2_DestroyActor`))

(fn `UserConstructionScript`)