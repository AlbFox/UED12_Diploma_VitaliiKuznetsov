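; Base interactable door that swings open and shut on Interact, with an optional lock cleared by a named key in the player's pickup storage.
; A state machine gates input, and unlocking only sets Closed, so opening takes another interaction.
; A timeline, timed by DoorTimelineSpeed as a divisor, drives 90-degree yaw while collision is off.
; A dot product against the player's position picks the swing direction on opening.
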(event `self.ReceiveBeginPlay`
  (bind _doortimelinespeed (`self.DoorTimelineSpeed`))
  (`TimelineComponent.SetPlayRate` (`self.OpenDoor`) (/ 1.0 (`KismetMathLibrary.SelectFloat` _doortimelinespeed 1.0 (!= _doortimelinespeed 0.0)))))

(event `/Game/Blueprints/Interactives/BPI_Interactions.Interact`
  (bind _door (`self.Door`))
  (`self.Interacted`)
  (switch `/Game/Blueprints/Interactives/E_DoorStates` (`self.DoorStates`)
    (:`NewEnumerator0`
      (bind _asbp_player_character (cast `/Game/Player/Blueprints/BP_PlayerCharacter` (`GameplayStatics.GetPlayerCharacter` 0)))
      (if (`/Game/Blueprints/PickUps/Comp_PickupsStorage.CheckPickupByName` (`/Game/Player/Blueprints/BP_PlayerCharacter.Comp_PickupsStorage` _asbp_player_character) (`self.KeyName`))
        (set `self.DoorStates` "NewEnumerator1")))
    (:`NewEnumerator1`
      (set `self.DoorStates` "NewEnumerator3")
      (`PrimitiveComponent.SetCollisionEnabled` _door "NoCollision")
      (set `self.DotProduct` (`self.MakeDotProduct`))
      (bind (_direction _alpha) (`Timeline|OpenDoor` :!label _label)
        (:`Update`
          (`SceneComponent.K2_SetRelativeRotation` (`self.Door`) (`self.MakeDoorRotation` _alpha) false false))
        (:`Finished`
          (switch `ETimelineDirection` _direction
            (:`Forward`
              (set `self.DoorStates` "NewEnumerator2"))
            (:`Backward`
              (set `self.DoorStates` "NewEnumerator1")))
          (`PrimitiveComponent.SetCollisionEnabled` (`self.Door`) "QueryAndPhysics"))))
    (:`NewEnumerator2`
      (set `self.DoorStates` "NewEnumerator3")
      (`PrimitiveComponent.SetCollisionEnabled` _door "NoCollision")
      (goto _label :!via `Reverse`))))

(fn `MakeDoorRotation`
  (params (Alpha :type "Float (double-precision)"))
  (returns (ReturnValue :type "Rotator Structure"))
  (return (`KismetMathLibrary.MakeRotator` 0.0 0.0 (`KismetMathLibrary.Lerp` 0.0 (`KismetMathLibrary.SelectFloat` 90.0 -90.0 (<= (`self.DotProduct`) 0.0)) Alpha))))

(fn `MakeDotProduct`
  (returns (ReturnValue :type "Float (double-precision)"))
  (bind _door (`self.Door`))
  (return (`KismetMathLibrary.Dot_VectorVector` (`KismetMathLibrary.Normal` (- (`SceneComponent.K2_GetComponentLocation` _door) (`self.K2_GetActorLocation` (`GameplayStatics.GetPlayerCharacter` 0)))) (`SceneComponent.GetRightVector` _door))))

(fn `UserConstructionScript`
  (`PrimitiveComponent.SetMaterial` (`self.Door`) 0 (`self.MeshMaterial`)))