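; Interactable weapon pickup actor that hands its weapon type to the player's weapon component when used.
; Interact passes the type and itself to SetCurrentWeapon on BP_PlayerCharacter, and ChangePickupWeapon lets the pickup switch to another weapon type.
; The construction script and type changes both look up the DT_Weapons row for the type and apply its static mesh to the pickup mesh.
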(event `/Game/Blueprints/Interactives/BPI_Interactions.Interact`
  (bind _asbp_player_character (cast `/Game/Player/Blueprints/BP_PlayerCharacter` (`GameplayStatics.GetPlayerCharacter` 0)))
  (`/Game/Blueprints/Components/Weapon/Comp_Weapon.SetCurrentWeapon` (`/Game/Player/Blueprints/BP_PlayerCharacter.Comp_Weapon` _asbp_player_character) (`self.WeaponType`) self))

(event `ChangePickupWeapon`
  (params (NewWeapon :type "/Game/Blueprints/Components/Weapon/E_WeaponType Enum" :default "NewEnumerator2"))
  (set `self.WeaponType` NewWeapon)
  (`self.SetStaticMesh`))

(fn `SetStaticMesh`
  (bind _returnvalue (`|GetDataTableRow` "/Game/Blueprints/Components/Weapon/DT_Weapons.DT_Weapons" (select `/Game/Blueprints/Components/Weapon/E_WeaponType` (`self.WeaponType`) :`NewEnumerator2` "Pistol" :`NewEnumerator0` "ShortGun" :`NewEnumerator1` "Rifle" :`NewEnumerator3` "RocketLauncher" :`NewEnumerator4` "SniperRifle" :!type "Name"))
    (:`then`
      (`StaticMeshComponent.SetStaticMesh` (`self.PickupMesh`) (`.StaticMesh_8_92EA30D74B35122F5C8E4DA6A772DBDD` (break `/Game/Blueprints/Components/Weapon/Str_Weapons` _returnvalue))))))

(fn `UserConstructionScript`
  (`parent.UserConstructionScript`)
  (`self.SetStaticMesh`))