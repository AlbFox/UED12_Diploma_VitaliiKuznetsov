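; Base player weapon that fires projectile bullets from its muzzle, with optional autofire on a looping timer.
; Each shot plays a sound by weapon type, spawns the configured bullets and starts a fire-rate cooldown tracked as IsReloading.
; Bullets head toward a camera line-trace point, using a random cone narrowed while aiming.
; In multi-bullet shots, the first bullet skips the spread and follows the camera center.
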(event `self.ReceiveBeginPlay`
  (bind _asbp_player_character (cast `/Game/Player/Blueprints/BP_PlayerCharacter` (`GameplayStatics.GetPlayerCharacter` 0)))
  (set `self.PlayerCharacter` _asbp_player_character))

(event `StopShooting`
  (`KismetSystemLibrary.K2_ClearAndInvalidateTimerHandle` (`self.SpawnShotHandle`)))

(event `MakeShot`
  (if (not (`self.IsReloading`))
    (`self.SpawnShot`)
    (if (`self.CanDoAutofire?`)
      (bind _returnvalue (`KismetSystemLibrary.K2_SetTimerDelegate` (`|CreateDelegate` :!event `SpawnShot`) (`self.CalculateFireRate` (`.AttacksPerSecond_2_DB57C88D4ED29087BF49F99CDCB5527A` (break `/Game/Blueprints/Components/Weapon/Str_AttackParameters` (`self.AttackParameters`)))) true))
      (set `self.SpawnShotHandle` _returnvalue))))

(fn `CalculateBulletDirection`
  (params (IsFirstBullet :type Boolean))
  (returns (SpreadLocation :type "Vector Structure"))
  (locals (L_IsFirstBullet :type Boolean) (L_TraceEnd :type "Vector Structure" :default (0.0 0.0 0.0)) (L_TargetPoint :type "Vector Structure" :default (0.0 0.0 0.0)))
  (bind ((`BulletClass_24_3D099DC347AA82F127A5899C23DDE503` _bulletclass) (`MaxSpread_17_6097731E47F24CAFE8117EBA5E8CA805` _maxspread) (`MinSpread_20_80A0F1E2473D157BD7023A854A4BD5CE` _minspread)) (break `/Game/Blueprints/Components/Weapon/Str_AttackParameters` (`self.AttackParameters`)))
  (set `local.L_IsFirstBullet` IsFirstBullet)
  (bind _desiredview (`CameraComponent.GetCameraView` (`/Game/Player/Blueprints/BP_PlayerCharacter.Camera` (`self.PlayerCharacter`)) 0.0))
  (if (`local.L_IsFirstBullet`)
    (bind (_location _rotation) (break `MinimalViewInfo` _desiredview))
    (bind _returnvalue (`KismetMathLibrary.GetForwardVector` _rotation))
    (set `local.L_TraceEnd` (+ _location (* (`KismetMathLibrary.RandomUnitVectorInConeInDegrees` _returnvalue (* (select `bool` (`/Game/Player/Blueprints/BP_PlayerCharacter.IsAiming` (`self.PlayerCharacter`)) :`false` _maxspread :`true` _minspread) 0.5)) (`self.ForwardLength`))))
    (else
      (bind _returnvalue_2 (+ _location (* _returnvalue (`self.ForwardLength`))))
      (set `local.L_TraceEnd` _returnvalue_2)))
  (bind _outhit (`KismetSystemLibrary.LineTraceSingle` _location (`local.L_TraceEnd`) "TraceTypeQuery1"))
  (bind (_bblockinghit _binitialoverlap _time _distance _location_2) (`GameplayStatics.BreakHitResult` _outhit))
  (if _bblockinghit
    (set `local.L_TargetPoint` _location_2)
    (else
      (set `local.L_TargetPoint` _returnvalue_2)))
  (return (`KismetMathLibrary.Normal` (- (`local.L_TargetPoint`) (`SceneComponent.K2_GetComponentLocation` (`self.SComp_Muzzle`))))))

(fn `CalculateFireRate`
  (params (AttacksPerSecond :type "Float (double-precision)"))
  (returns (ReturnValue :type "Float (double-precision)"))
  (if (!= AttacksPerSecond 0.0)
    (return (/ 1.0 AttacksPerSecond))))

(fn `CalculateSpread`
  (params (VectorToModify :type "Vector Structure"))
  (returns (ModifiedVector :type "Vector Structure"))
  (return (`KismetMathLibrary.MakeVector` (+ (.x VectorToModify) (`self.GetSpread`)) (+ (.y VectorToModify) (`self.GetSpread`)) (+ (.z VectorToModify) (`self.GetSpread`)))))

(fn `FirstBulletCheck`
  (params (BulletIndex :type Integer) (BulletsPerShot :type Integer))
  (returns (ReturnValue :type Boolean))
  (return (or (!= BulletIndex 1) (== BulletsPerShot 1))))

(fn `GetSpread`
  (returns (RandomSpread :type "Float (double-precision)"))
  (bind _returnvalue (* (+ (`.MaxSpread_17_6097731E47F24CAFE8117EBA5E8CA805` (break `/Game/Blueprints/Components/Weapon/Str_AttackParameters` (`self.AttackParameters`))) (`KismetMathLibrary.SelectFloat` 0.0 90.0 (`/Game/Player/Blueprints/BP_PlayerCharacter.IsAiming` (`self.PlayerCharacter`)))) 0.5))
  (return (`KismetMathLibrary.RandomFloatInRange` (* _returnvalue -1.0) _returnvalue)))

(fn `Reloading`
  (set `self.IsReloading` false))

(fn `SetComponentWeapon`
  (params (ComponentWeapon :type "/Game/Blueprints/Components/Weapon/Comp_Weapon Object Reference"))
  (set `self.ComponentWeapon` ComponentWeapon))

(fn `SpawnBullet`
  (params (AttackParameters :type "/Game/Blueprints/Components/Weapon/Str_AttackParameters Structure"))
  (locals (L_AttackParameters :type "/Game/Blueprints/Components/Weapon/Str_AttackParameters Structure"))
  (bind (_l_attackparameters_bulletclass _l_attackparameters_attackspersecond _l_attackparameters_maxspread _l_attackparameters_minspread _l_attackparameters_bulletspershot _l_attackparameters_damage _l_attackparameters_bulletspeed _l_attackparameters_bulletlifetime) (break `/Game/Blueprints/Components/Weapon/Str_AttackParameters` (`local.L_AttackParameters`)))
  (set `local.L_AttackParameters` AttackParameters)
  (for _index (range 1 (+ _l_attackparameters_bulletspershot 1))
    (`|SpawnActorFromClass` _l_attackparameters_bulletclass (`KismetMathLibrary.MakeTransform` (`SceneComponent.K2_GetComponentLocation` (`self.SComp_Muzzle`)) (struct) (0.4 0.4 0.4)) "Undefined" "OverrideRootScale" null _l_attackparameters_damage _l_attackparameters_bulletspeed _l_attackparameters_bulletlifetime (`self.CalculateBulletDirection` (`self.FirstBulletCheck` _index _l_attackparameters_bulletspershot)) null)))

(fn `SpawnShot`
  (bind _attackparameters (`self.AttackParameters`))
  (`GameplayStatics.PlaySoundAtLocation` (select `/Game/Blueprints/Components/Weapon/E_WeaponType` (`self.WeaponType`) :`NewEnumerator0` "/Game/Sound/Weapons/S_ShotgunShot.S_ShotgunShot" :`NewEnumerator1` "/Game/Sound/Weapons/S_RifleShot.S_RifleShot" :`NewEnumerator3` "/Game/Sound/Weapons/S_RocketLauncher.S_RocketLauncher" :`NewEnumerator4` "/Game/Sound/Weapons/S_SniperRifle.S_SniperRifle" :!type "SoundBase Object Reference") (`SceneComponent.K2_GetComponentLocation` (`self.SComp_Muzzle`)) (struct) 1.0 1.0 0.0 null null null)
  (`self.SpawnBullet` _attackparameters)
  (set `self.IsReloading` true)
  (`KismetSystemLibrary.K2_SetTimerDelegate` (`|CreateDelegate` :!event `Reloading`) (`self.CalculateFireRate` (`.AttacksPerSecond_2_DB57C88D4ED29087BF49F99CDCB5527A` (break `/Game/Blueprints/Components/Weapon/Str_AttackParameters` _attackparameters)))))

(fn `UserConstructionScript`)