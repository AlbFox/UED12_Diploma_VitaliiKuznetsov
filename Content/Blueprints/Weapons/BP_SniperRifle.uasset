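; Sniper rifle weapon Blueprint that fires hitscan shots dealing fixed damage.
; SpawnShot spends ammo through the weapon component, calls SpawnBullet, then sets IsReloading and starts a fire-rate timer.
; SpawnBullet traces from the muzzle toward the point found by a camera trace, so shots follow the player's aim, and sends damage to the hit actor.
; The muzzle trace draws persistent debug lines; CalculateHitscanEnd is not called here.
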(fn `CalculateEndTrace`
  (returns (EndTraceLocation :type "Vector Structure"))
  (bind _camera (`/Game/Player/Blueprints/BP_PlayerCharacter.Camera` (`self.PlayerCharacter`)))
  (bind _returnvalue (`SceneComponent.K2_GetComponentLocation` _camera))
  (bind _returnvalue_2 (+ _returnvalue (* (`SceneComponent.GetForwardVector` _camera) (`self.ForwardLength`))))
  (bind (_outhit _returnvalue_3) (`KismetSystemLibrary.LineTraceSingle` :`Start` _returnvalue :`End` _returnvalue_2 :`TraceChannel` "TraceTypeQuery3" :`DrawTime` 0.0))
  (if _returnvalue_3
    (return (`.ImpactPoint` (`GameplayStatics.BreakHitResult` _outhit)))
    (else
      (return _returnvalue_2))))

(fn `CalculateHitscanEnd`
  (returns (ReturnValue :type "Vector Structure"))
  (bind _desiredview (`CameraComponent.GetCameraView` (`/Game/Player/Blueprints/BP_PlayerCharacter.Camera` (`self.PlayerCharacter`)) 0.0))
  (bind (_location _rotation) (break `MinimalViewInfo` _desiredview))
  (return (+ _location (* (`KismetMathLibrary.GetForwardVector` _rotation) (`self.ForwardLength`)))))

(fn `SpawnBullet`
  (params (AttackParameters :type "/Game/Blueprints/Components/Weapon/Str_AttackParameters Structure"))
  (locals (L_AttackParameters :type "/Game/Blueprints/Components/Weapon/Str_AttackParameters Structure"))
  (set `local.L_AttackParameters` AttackParameters)
  (bind (_outhit _returnvalue) (`KismetSystemLibrary.LineTraceSingle` :`Start` (`SceneComponent.K2_GetComponentLocation` (`self.SComp_Muzzle`)) :`End` (`self.CalculateEndTrace`) :`TraceChannel` "TraceTypeQuery3" :`DrawDebugType` "Persistent" :`DrawTime` 0.0))
  (if _returnvalue
    (message `/Game/Blueprints/Components/Parameters/BPI_Damage.DealDamage` (`.HitActor` (`GameplayStatics.BreakHitResult` _outhit)) 100)))

(fn `SpawnShot`
  (bind _attackparameters (`self.AttackParameters`))
  (bind _hasammo_ (`/Game/Blueprints/Components/Weapon/Comp_Weapon.DecreaseWeaponCurrentAmmo` (`self.ComponentWeapon`) (`self.WeaponType`)))
  (if _hasammo_
    (`self.SpawnBullet` _attackparameters)
    (set `self.IsReloading` true)
    (`KismetSystemLibrary.K2_SetTimerDelegate` (`|CreateDelegate` :!event `Reloading`) (`self.CalculateFireRate` (`.AttacksPerSecond_2_DB57C88D4ED29087BF49F99CDCB5527A` (break `/Game/Blueprints/Components/Weapon/Str_AttackParameters` _attackparameters))))))

(fn `UserConstructionScript`
  (`parent.UserConstructionScript`))