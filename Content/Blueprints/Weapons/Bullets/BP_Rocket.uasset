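; BP_Rocket is a bullet actor for a rocket weapon that speeds up in flight and explodes.
; Tick multiplies the projectile movement velocity by a constant every frame, giving compounding, frame-rate-dependent acceleration.
; A collision overlap or the end of its lifetime delay calls SpawnExplosion, which spawns BP_RocketExplosion at the rocket's transform and destroys the rocket.
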(event `self.ReceiveTick`
  (params (DeltaSeconds :type "Float (single-precision)"))
  (bind _projectilemovement (`self.ProjectileMovement`))
  (set `MovementComponent.Velocity` (* (`MovementComponent.Velocity` _projectilemovement) 1.05) _projectilemovement))

(event `self.ReceiveBeginPlay`
  (`KismetSystemLibrary.Delay` (`self.Lifetime`))
  (`self.SpawnExplosion`))

(event `self.BulletCollision.OnComponentBeginOverlap`
  (params (OverlappedComponent :type "PrimitiveComponent Object Reference") (OtherActor :type "Actor Object Reference") (OtherComp :type "PrimitiveComponent Object Reference") (OtherBodyIndex :type Integer) (bFromSweep :type Boolean) (SweepResult :type "HitResult Structure (by ref)"))
  (`self.SpawnExplosion`))

(fn `SpawnExplosion`
  (`|SpawnActorFromClass` "/Game/Blueprints/DamageVolumes/BP_RocketExplosion.BP_RocketExplosion_C" (`self.GetTransform`) "Undefined" "OverrideRootScale" null null)
  (`self.K2_DestroyActor`))

(fn `UserConstructionScript`
  (`parent.UserConstructionScript`))