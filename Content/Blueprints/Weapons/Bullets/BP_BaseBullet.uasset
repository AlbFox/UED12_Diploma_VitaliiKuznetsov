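; BP_BaseBullet is a base projectile actor for weapons that damages what it hits.
; The construction script sets the ProjectileMovement initial speed and velocity from its InitialSpeed and Direction variables.
; On collision overlap, it sends a DealDamage message with its Damage value to the other actor, then destroys itself.
; A delay started at BeginPlay destroys it once Lifetime expires.
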(event `self.ReceiveBeginPlay`
  (`KismetSystemLibrary.Delay` (`self.Lifetime`))
  (`self.K2_DestroyActor`))

(event `self.BulletCollision.OnComponentBeginOverlap`
  (params (OverlappedComponent :type "PrimitiveComponent Object Reference") (OtherActor :type "Actor Object Reference") (OtherComp :type "PrimitiveComponent Object Reference") (OtherBodyIndex :type Integer) (bFromSweep :type Boolean) (SweepResult :type "HitResult Structure (by ref)"))
  (message `/Game/Blueprints/Components/Parameters/BPI_Damage.DealDamage` OtherActor (`self.Damage`))
  (`self.K2_DestroyActor`))

(fn `UserConstructionScript`
  (bind _projectilemovement (`self.ProjectileMovement`))
  (bind _output_get (set `ProjectileMovementComponent.InitialSpeed` (`self.InitialSpeed`) _projectilemovement))
  (set `MovementComponent.Velocity` (* (`self.Direction`) _output_get) _projectilemovement))