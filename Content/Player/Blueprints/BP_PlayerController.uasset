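; Player controller that manages the game's UI screens: main screen, HUD, defeat and victory.
; BeginPlay opens the main screen with UI-only input, and StartGame switches to the HUD with game-only input.
; A CurrentWidget reference tracks the active screen, which each transition removes before adding the next, toggling the mouse cursor.
; Retry reopens Map_Level_1 and re-adds the stored HUD, and an ExitGame event handles exiting.
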(event `self.ReceiveBeginPlay`
  ;[1 1 1] Begin play
  (bind _returnvalue (`|CreateWidget` "/Game/UserInterface/W_MainScreen.W_MainScreen_C"))
  (bind _output_get (set `self.CurrentWidget` _returnvalue))
  (`UserWidget.AddToViewport` _output_get 0)
  (`WidgetBlueprintLibrary.SetInputMode_UIOnlyEx` self null)
  (set `self.bShowMouseCursor` true))

(event `StartGame`
  ;[1 1 1] Begin play
  (`Widget.RemoveFromParent` (`self.CurrentWidget`))
  (bind _returnvalue (`|CreateWidget` "/Game/UserInterface/W_Screen_HUD.W_Screen_HUD_C"))
  (bind _output_get (set `self.HUD` _returnvalue))
  (bind _output_get_2 (set `self.CurrentWidget` _output_get))
  (`UserWidget.AddToViewport` _output_get_2 0)
  (`WidgetBlueprintLibrary.SetInputMode_GameOnly` self)
  (set `self.bShowMouseCursor` false))

(event `ExitGame`
  ;[1 1 1] Main screen functions
  (`self.ExitGame`))

(event `Retry`
  (bind _hud (`self.HUD`))
  ;[1 1 1] Main screen functions
  (`Widget.RemoveFromParent` (`self.CurrentWidget`))
  (`GameplayStatics.OpenLevel` "Map_Level_1")
  (set `self.CurrentWidget` _hud)
  (`UserWidget.AddToViewport` _hud 0)
  (set `self.bShowMouseCursor` false))

(fn `AddDefeatScreen`
  (`Widget.RemoveFromParent` (`self.CurrentWidget`))
  (bind _returnvalue (`|CreateWidget` "/Game/UserInterface/W_DefeatScreen.W_DefeatScreen_C"))
  (bind _output_get (set `self.DefeatScreen` _returnvalue))
  (bind _output_get_2 (set `self.CurrentWidget` _output_get))
  (`UserWidget.AddToViewport` _output_get_2 0)
  (set `self.bShowMouseCursor` true))

(fn `AddVictoryScreen`
  (`Widget.RemoveFromParent` (`self.CurrentWidget`))
  (bind _returnvalue (`|CreateWidget` "/Game/UserInterface/W_VictoryScreen.W_VictoryScreen_C"))
  (bind _output_get (set `self.VictoryScreen` _returnvalue))
  (bind _output_get_2 (set `self.CurrentWidget` _output_get))
  (`UserWidget.AddToViewport` _output_get_2 0)
  (set `self.bShowMouseCursor` true))

(fn `UserConstructionScript`)