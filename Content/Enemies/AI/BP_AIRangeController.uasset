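; AI controller for ranged enemies that runs the BT_RangeEnemy behavior tree and handles their switch to aggression.
; On BeginPlay it seeds the blackboard with the pawn's start location and an initial EnemyState, then caches the pawn as a base enemy.
; Tick polls the distance to the player, and within a fixed radius SetAgressiveState writes the player and a new state to the blackboard, latched once by WasAgro.
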(event `self.ReceiveTick`
  (params (DeltaSeconds :type "Float (single-precision)"))
  (if (not (`self.WasAgro`))
    (bind _asbp_player_character (cast `/Game/Player/Blueprints/BP_PlayerCharacter` (`GameplayStatics.GetPlayerCharacter` 0)))
    (`/Engine/EditorBlueprintResources/StandardMacros.IsValid` _asbp_player_character
      (:`Is Valid`
        (if (< (`KismetMathLibrary.VSize` (- (`self.K2_GetActorLocation` _asbp_player_character) (`self.K2_GetActorLocation` (`self.Enemy`)))) 1000.0)
          (`self.SetAgressiveState`))))))

(event `self.ReceiveBeginPlay`
  (`self.RunBehaviorTree` "/Game/Enemies/AI/BT_RangeEnemy.BT_RangeEnemy")
  (`BlackboardComponent.SetValueAsVector` (`self.Blackboard`) "InitialLocation" (`self.K2_GetActorLocation` (`self.K2_GetPawn`)))
  (`BlackboardComponent.SetValueAsEnum` (`self.Blackboard`) "EnemyState" (enumliteral `/Game/Enemies/AI/E_EnemyState` "NewEnumerator0"))
  (bind _asbp_base_enemy_character (cast `/Game/Enemies/Characters/BP_BaseEnemyCharacter` (`self.K2_GetPawn`)))
  (set `self.Enemy` _asbp_base_enemy_character))

(event `SetAgressiveState`
  (if (not (`self.WasAgro`))
    (set `self.WasAgro` true)
    (bind _asbp_player_character (cast `/Game/Player/Blueprints/BP_PlayerCharacter` (`GameplayStatics.GetPlayerCharacter` 0)))
    (`BlackboardComponent.SetValueAsObject` (`self.Blackboard`) "Player" _asbp_player_character)
    (`BlackboardComponent.SetValueAsEnum` (`self.Blackboard`) "EnemyState" (enumliteral `/Game/Enemies/AI/E_EnemyState` "NewEnumerator2"))))

(fn `UserConstructionScript`)