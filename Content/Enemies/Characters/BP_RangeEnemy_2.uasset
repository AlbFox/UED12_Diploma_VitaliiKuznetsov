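; BP_RangeEnemy_2 is a ranged enemy variant whose attack fires a burst of five damage orbs at the player.
; The Attack event calls SpawnBullet repeatedly with a short delay between shots.
; Each SpawnBullet spawns a BP_DamageOrb at the enemy's location, rotated toward player character 0's current position, so every shot re-aims as the burst plays out.
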(event `self.Attack`
  (`self.SpawnBullet`)
  (`KismetSystemLibrary.Delay` 0.2)
  (`self.SpawnBullet`)
  (`KismetSystemLibrary.Delay` 0.2)
  (`self.SpawnBullet`)
  (`KismetSystemLibrary.Delay` 0.2)
  (`self.SpawnBullet`)
  (`KismetSystemLibrary.Delay` 0.2)
  (`self.SpawnBullet`)
  (`KismetSystemLibrary.Delay` 0.2))

(fn `SpawnBullet`
  (bind (_returnvalue_roll _returnvalue_pitch _returnvalue_yaw) (`KismetMathLibrary.BreakRotator` (`KismetMathLibrary.FindLookAtRotation` (`self.K2_GetActorLocation`) (`self.K2_GetActorLocation` (`GameplayStatics.GetPlayerCharacter` 0)))))
  (`|SpawnActorFromClass` "/Game/Enemies/DamageOrbs/BP_DamageOrb.BP_DamageOrb_C" (`KismetMathLibrary.MakeTransform` (`self.K2_GetActorLocation`) (`KismetMathLibrary.MakeRotator` _returnvalue_roll _returnvalue_pitch _returnvalue_yaw)) "Undefined" "OverrideRootScale" null null))

(fn `UserConstructionScript`
  (`parent.UserConstructionScript`))