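; BP_BaseEnemyCharacter is the base enemy character, with health, a montage-driven melee attack and ragdoll death.
; DealDamage passes damage to the parameters component, whose Death event flags the enemy dead, disables capsule collision and enables mesh physics.
; DamageCollision overlaps damage the player while IsAttacking, guarded by WasHit, though neither IsAttacking nor a WasHit reset is set here.
; Debug prints show damage received and attack flags every tick.
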(event `self.ReceiveBeginPlay`
  (`/Game/Blueprints/Components/Parameters/Comp_Parameters.SetCurrentHealth` (`self.Comp_Parameters`) 100))

(event `/Game/Blueprints/Components/Parameters/BPI_Damage.DealDamage`
  (params (Damage :type Integer))
  (`/Game/Blueprints/Components/Parameters/Comp_Parameters.ApplyDamageToParameters` (`self.Comp_Parameters`) Damage)
  (`KismetSystemLibrary.PrintString` (`KismetStringLibrary.Conv_IntToString` Damage)))

(event `self.Comp_Parameters.Death`
  (set `self.IsDead` true)
  (`self.Death`))

(event `Attack`
  (`self.PlayAnimMontage` "/Game/Enemies/Characters/Animation/Attack/Anim_Infected_Attack_1_Montage.Anim_Infected_Attack_1_Montage"))

(event `self.DamageCollision.OnComponentBeginOverlap`
  (params (OverlappedComponent :type "PrimitiveComponent Object Reference") (OtherActor :type "Actor Object Reference") (OtherComp :type "PrimitiveComponent Object Reference") (OtherBodyIndex :type Integer) (bFromSweep :type Boolean) (SweepResult :type "HitResult Structure (by ref)"))
  (if (and (`self.IsAttacking`) (not (`self.WasHit`)))
    (set `self.WasHit` true)
    (bind _asbp_player_character (cast `/Game/Player/Blueprints/BP_PlayerCharacter` OtherActor))
    (`/Game/Blueprints/Components/Parameters/BPI_Damage.DealDamage` _asbp_player_character 30)))

(event `self.ReceiveTick`
  (params (DeltaSeconds :type "Float (single-precision)"))
  (`KismetSystemLibrary.PrintString` (`KismetStringLibrary.Conv_BoolToString` (`self.IsAttacking`)) true true (struct :`G` 1.0 :`B` 0.950161 :`A` 1.0) 0.0)
  (`KismetSystemLibrary.PrintString` (`KismetStringLibrary.Conv_BoolToString` (`self.WasHit`)) true true (struct :`R` 0.005358 :`G` 1.0 :`A` 1.0) 0.0))

(fn `Death`
  (`PrimitiveComponent.SetCollisionEnabled` (`self.CapsuleComponent`) "NoCollision")
  (`PrimitiveComponent.SetCollisionEnabled` (`self.Mesh`) "PhysicsOnly")
  (`PrimitiveComponent.SetSimulatePhysics` (`self.Mesh`) true)
  (`PrimitiveComponent.SetCollisionResponseToAllChannels` (`self.Mesh`) "ECR_Block"))

(fn `UserConstructionScript`)