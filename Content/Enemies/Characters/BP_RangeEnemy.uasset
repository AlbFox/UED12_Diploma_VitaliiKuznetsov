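; BP_RangeEnemy is a ranged enemy whose attack fires a spread of BP_DamageOrb projectiles.
; The Attack event loops over the Shots count, spawning each orb at the actor's location with yaw offset from its facing by multiples of Angle.
; Indices from half of Shots upward have Shots subtracted, fanning orbs to both sides of forward without sorting.
; The construction script only calls the parent's.
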(event `self.Attack`
  (bind _index (`self.Index`))
  (for _index_2 (range 1 (+ (`self.Shots`) 1))
    (set `self.Index` _index_2)
    (`|SpawnActorFromClass` "/Game/Enemies/DamageOrbs/BP_DamageOrb.BP_DamageOrb_C" (`KismetMathLibrary.MakeTransform` (`self.K2_GetActorLocation`) (`KismetMathLibrary.MakeRotator` 0.0 0.0 (+ (.yaw (`self.K2_GetActorRotation`)) (* (`KismetMathLibrary.SelectInt` (- _index (`self.Shots`)) _index (>= _index (/ (`self.Shots`) 2))) (`self.Angle`))))) "Undefined" "OverrideRootScale" null null)))

(fn `UserConstructionScript`
  (`parent.UserConstructionScript`))